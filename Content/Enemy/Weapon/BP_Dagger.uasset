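; BP_Dagger is an enemy melee weapon that resolves hits on the player when its collision begins overlapping.
; Overlaps count only while the owning BP_Enemy is attacking, outside one excluded state, and not flagged as hit.
; The player's parry takes priority over defend, each triggering its success handler on the player.
; Otherwise it applies fixed damage through the player's damage system and updates the HUD health percentage.
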(event Collision|EventActorBeginOverlap
  (params (OtherActor :type Actor%20Object%20Reference))
  (bind _asbp_enemy (Utilities|Casting|CastToBP_Enemy (Components|GetOwner)))
  (bind _output_get (Variables|Default|SetAs%20BP%20Enemy _asbp_enemy))
  (if (Math|Boolean|ANDBoolean (Variables|/Game/Enemy/BP_Enemy.BP_Enemy_C|GetOnAttack _output_get) (Utilities|Enum|NotEqual(Enum) (Variables|/Game/Enemy/BP_Enemy.BP_Enemy_C|GetState _output_get) "NewEnumerator1") (not (Variables|/Game/Component/BP_DamageSystem.BP_DamageSystem_C|GetbHit (Variables|/Game/Enemy/BP_Enemy.BP_Enemy_C|GetBP_DamageSystem _output_get))))
    (bind _asbp_player (Utilities|Casting|CastToBP_Player OtherActor))
    (bind _output_get_2 (Variables|Default|SetPlayer _asbp_player))
    (if (Variables|/Game/Player/BP_Player.BP_Player_C|GetOnParry _output_get_2)
      (Default|ParrySuccess (Variables|Default|GetPlayer) (Variables|Default|GetAs%20BP%20Enemy))
      (elif (Variables|/Game/Player/BP_Player.BP_Player_C|GetOnDefend (Variables|Default|GetPlayer))
        (Default|DefendSuccess (Variables|Default|GetPlayer))
        (else
          (Default|GetDamage (Variables|/Game/Player/BP_Player.BP_Player_C|GetBP_DamageSystem (Variables|Default|GetPlayer)) 1.0 self)
          (Default|SetTargetPercent (Variables|/Game/Player/BP_Player.BP_Player_C|GetHUD (Variables|Default|GetPlayer)) (/ (Variables|/Game/Component/BP_DamageSystem.BP_DamageSystem_C|GetHealth%20Point (Variables|/Game/Player/BP_Player.BP_Player_C|GetBP_DamageSystem (Variables|Default|GetPlayer))) 1e+02)))))))

(event EventTick
  (params (DeltaSeconds :type Float%20%28single-precision%29)))

(fn ConstructionScript)