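; Dagger-wielding assassin enemy that detects, chases and attacks the player, with hit, stun and death handling.
; Tick runs a state machine driven by distance and BPDamageSystem flags; SetState mirrors state to the Blackboard and enables dagger collision only in Attack.
; Chase moves directly toward the player, using knee and eye traces to trigger parkour over low obstacles.
; Attacks pick montage sections from a seeded random stream; a viewport widget shows status.
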(event Custom|DaggerCollision
  (params (SetCollision :type Boolean))
  (Collision|SetActorEnableCollision (Variables|/Script/Engine.ChildActorComponent|GetChildActor (Variables|Default|GetLeftDagger)) SetCollision)
  (Collision|SetActorEnableCollision (Variables|/Script/Engine.ChildActorComponent|GetChildActor (Variables|Default|GetRightDagger)) SetCollision))

(event EventBeginPlay
  ;[1 1 1] 플레이어 기억
  (bind _asbp_player (Utilities|Casting|CastToBP_Player (Game|Player|GetPlayerPawn 0)))
  (Variables|Default|SetPlayer _asbp_player)
  (CallFunction|SetState "NewEnumerator2")
  ;[1 1 1] 랜덤 시드 생성
  (bind _output_get (Variables|Default|SetRandomSeed (Math|Random|MakeRandomStream 0)))
  (Math|Random|SetRandomStreamSeed _output_get (+ (* (Utilities|Time|GetGameTimeinSeconds) 1e+03) (Math|Random|RandomInteger 101)))
  ;[1 1 1] 칼 주인 설정
  (Actor|SetOwner (Variables|/Script/Engine.ChildActorComponent|GetChildActor (Variables|Default|GetLeftDagger)) self)
  (Actor|SetOwner (Variables|/Script/Engine.ChildActorComponent|GetChildActor (Variables|Default|GetRightDagger)) self)
  ;[1 1 1] 적 상태 UI
  (bind _returnvalue (UserInterface|CreateWidget "/Game/UI/WBP_EnemyStatus.WBP_EnemyStatus_C"))
  (bind _output_get_2 (Variables|Default|SetStatusUI _returnvalue))
  (Default|SetOwner _output_get_2 self)
  (UserInterface|Viewport|AddtoViewport (Variables|Default|GetStatusUI) 0)
  (Widget|SetVisibility (Variables|Default|GetStatusUI) "Hidden"))

(event EventTick
  (params (DeltaSeconds :type Float%20%28single-precision%29))
  (bind _bp_damagesystem (Variables|Default|GetBP_DamageSystem))
  (bind _mesh (Variables|Character|GetMesh))
  (bind _returnvalue (Components|SkeletalMesh|GetAnimInstance _mesh))
  ;[1 1 1] FSM
  (switch Utilities|FlowControl|Switch|SwitchonE_EnemyState (Variables|Default|GetState)
    (:NewEnumerator2
      (CallFunction|PatrolTick DeltaSeconds)
      ;[1 1 1] 죽음 상태 전환, 피격 애니메이션
      (if (Variables|/Game/Component/BP_DamageSystem.BP_DamageSystem_C|GetbDead _bp_damagesystem) :!label _label
        (Animation|StopAnimMontage "/Game/Enemy/Anim/DualBlade/AM_Hit.AM_Hit")
        (CallFunction|SetState "NewEnumerator1")
        (elif (Variables|/Game/Component/BP_DamageSystem.BP_DamageSystem_C|GetbHit _bp_damagesystem)
          (if (Animation|Montage|MontageIsPlaying _returnvalue "/Game/Enemy/Anim/DualBlade/AM_AssassinAttack.AM_AssassinAttack")
            (CallFunction|DaggerCollision false)
            (Ability|Animation|MontageJumptoSection _returnvalue "HIt" "/Game/Enemy/Anim/DualBlade/AM_AssassinAttack.AM_AssassinAttack")
            (Variables|/Game/Component/BP_DamageSystem.BP_DamageSystem_C|SetbHit (Variables|Default|GetBP_DamageSystem) false)))))
    (:NewEnumerator0
      (CallFunction|AttackTick DeltaSeconds)
      (goto _label))
    (:NewEnumerator1
      (CallFunction|DeadTick DeltaSeconds))
    (:NewEnumerator3
      (CallFunction|ChaseTick DeltaSeconds)
      (goto _label))
    (:NewEnumerator4
      (CallFunction|StunTick DeltaSeconds)
      (if (<= (Variables|Default|GetStunTime) 0.0)
        (CallFunction|SetState "NewEnumerator3")
        (Variables|Default|SetStunTime 3.0)
        (elif (Variables|/Game/Component/BP_DamageSystem.BP_DamageSystem_C|GetbHit (Variables|Default|GetBP_DamageSystem))
          (if (not (Animation|Montage|MontageIsPlaying (Components|SkeletalMesh|GetAnimInstance (Variables|Character|GetMesh)) "/Game/Enemy/Anim/DualBlade/AM_Hit.AM_Hit"))
            (Animation|PlayAnimMontage "/Game/Enemy/Anim/DualBlade/AM_Hit.AM_Hit" 1.0 "None")))))))

(fn ConstructionScript)

(fn AttackTick
  (params (DeltaTime :type Float%20%28double-precision%29))
  (if (not (Variables|Default|GetOnAttack))
    (LocalVariables|SetRandomIdx (Math|Random|RandomIntegerinRangefromStream (Variables|Default|GetRandomSeed) 1 7))
    (Animation|PlayAnimMontage "/Game/Enemy/Anim/DualBlade/AM_AssassinAttack.AM_AssassinAttack" 1.0 (Utilities|String|StringToName (Utilities|String|Append "Attack" (Utilities|String|ToString(Integer) (LocalVariables|GetRandomIdx)))))
    (Variables|Default|SetOnAttack true)))

(fn PatrolTick
  (params (DeltaTime :type Float%20%28double-precision%29))
  (Utilities|IsValid (Variables|Default|GetPlayer)
    (:Is%20Valid
      (if (< (Transformation|GetDistanceTo (Variables|Default|GetPlayer)) (Variables|Default|GetDetectRange))
        (CallFunction|SetState "NewEnumerator3")))))

(fn DeadTick
  (params (DeltaTime :type Float%20%28double-precision%29))
  (bind _mesh (Variables|Character|GetMesh))
  (bind _returnvalue (Components|SkeletalMesh|GetAnimInstance _mesh))
  (Class|AnimInstance|MontageStopwithBlendOut _returnvalue (Utilities|Struct|MakeAlphaBlendArgs 0 0.2 "Linear") "/Game/Enemy/Anim/DualBlade/AM_AssassinAttack.AM_AssassinAttack")
  (Class|AnimInstance|MontageStopwithBlendOut _returnvalue (Utilities|Struct|MakeAlphaBlendArgs 0 0.2 "Linear") "/Game/Enemy/Anim/AM_Parkour.AM_Parkour")
  (bind _output_get (Variables|Default|SetPostElapsedTime (- (Variables|Default|GetPostElapsedTime) DeltaTime)))
  (if (<= _output_get 0.0)
    (Collision|SetCollisionEnabled (Variables|Collision|GetCapsuleComponent) "NoCollision")))

(fn ChaseTick
  (params (DeltaTime :type Float%20%28double-precision%29))
  (bind _hitlocation (Variables|Default|GetHitLocation))
  (bind _player (Variables|Default|GetPlayer))
  (bind _returnvalue (Transformation|GetActorLocation _player))
  (bind _canover (CallFunction|DetectObstacle))
  (if _canover
    (if (not (Variables|Default|GetbOnce))
      (Variables|Default|SetbOnce true)
      (Character|Jump)
      (Variables|Default|SetOnParkour true)
      (Rendering|Debug|DrawDebugLine _hitlocation _returnvalue "(R=0.000000,G=1.000000,B=1.000000,A=1.000000)" 0.0 0.0)
      (AI|Components|Blackboard|SetValueasVector (AI|GetBlackboard (AI|GetAIController self)) (LocalVariables|GetTargetLocationKey) (- _returnvalue _hitlocation))
      (Animation|PlayAnimMontage "/Game/Enemy/Anim/AM_Parkour.AM_Parkour" 1.0 "None"))
    (elif (not (Variables|Default|GetOnParkour))
      (Utilities|IsValid (Variables|Default|GetPlayer)
        (:Is%20Valid
          (bind _output_get (Variables|Default|SetDirection (Math|Vector|Normalize (- (Transformation|GetActorLocation (Variables|Default|GetPlayer)) (Transformation|GetActorLocation self)))))
          (Pawn|Input|AddMovementInput _output_get (Variables|Default|GetSpeed) false)
          (CallFunction|TurntoTarget)
          (if (< (Transformation|GetDistanceTo (Variables|Default|GetPlayer)) (Variables|Default|GetAttackRange))
            (CallFunction|SetState "NewEnumerator0")
            (elif (> (Transformation|GetDistanceTo (Variables|Default|GetPlayer)) (Variables|Default|GetDetectRange))
              (CallFunction|SetState "NewEnumerator2"))))))))

(fn SetState
  (params (StateValue :type E_EnemyState%20Enum :default "NewEnumerator0"))
  (if (Utilities|Enum|Equal(Enum) StateValue "NewEnumerator1")
    (bind _statusui (Variables|Default|GetStatusUI)
      (:then
        (Widget|RemovefromParent _statusui))
      (:else)))
  (if (Utilities|Enum|NotEqual(Enum) (Variables|Default|GetState) StateValue)
    (if (Utilities|Enum|NotEqual(Enum) (Variables|Default|GetState) "NewEnumerator1")
      (bind _output_get (Variables|Default|SetState StateValue))
      (AI|Components|Blackboard|SetValueasEnum (AI|GetBlackboard (AI|GetAIController self)) (Variables|Default|GetEnemyStateKey) _output_get)
      (CallFunction|DaggerCollision (Utilities|Enum|Equal(Enum) (Variables|Default|GetState) "NewEnumerator0")))))

(fn TurntoTarget
  (Transformation|SetActorRotation (Math|Rotator|FindLookatRotation (Transformation|GetActorLocation) (Transformation|GetActorLocation (Variables|Default|GetPlayer)))))

(fn DetectObstacle
  (bind (_outhit _returnvalue) (Collision|LineTraceByChannel (Transformation|GetWorldLocation (Variables|Default|GetKneePoint)) (+ (Transformation|GetWorldLocation (Variables|Default|GetKneePoint)) (* (Math|Vector|GetForwardVector (Variables|Default|GetKneePoint)) 2e+02)) "TraceTypeQuery1" false 0 "None" true "(R=1.000000,G=0.000000,B=0.936080,A=1.000000)"))
  (Variables|Default|SetHitLocation (Transformation|GetActorLocation))
  (Utilities|Casting|CastToBP_Player (.hitactor _outhit)
    (:then
      (return false))
    (:CastFailed
      (bind _returnvalue_2 (Collision|LineTraceByChannel (Transformation|GetWorldLocation (Variables|Default|GetEyesPoint)) (+ (Transformation|GetWorldLocation (Variables|Default|GetEyesPoint)) (* (Math|Vector|GetForwardVector (Variables|Default|GetEyesPoint)) 2e+02)) "TraceTypeQuery1" false 0 "None"))
      (return (and (== _returnvalue_2 false) (== _returnvalue true))))))

(fn StunTick
  (params (DeltaTime :type Float%20%28double-precision%29))
  (bind _mesh (Variables|Character|GetMesh))
  (bind _returnvalue (Components|SkeletalMesh|GetAnimInstance _mesh))
  (bind _asabp_enemy (Utilities|Casting|CastToABP_Enemy _returnvalue))
  (Variables|/Game/Enemy/Anim/ABP_Enemy.ABP_Enemy_C|SetVelocity _asabp_enemy "0, 0, 0")
  (if (Animation|Montage|MontageIsPlaying _returnvalue "/Game/Enemy/Anim/DualBlade/AM_AssassinAttack.AM_AssassinAttack")
    (Animation|Montage|MontageStop _returnvalue 0.0 "/Game/Enemy/Anim/DualBlade/AM_AssassinAttack.AM_AssassinAttack"))
  (Variables|Default|SetStunTime (- (Variables|Default|GetStunTime) DeltaTime)))

(fn UIOrder
  (params (Visiblity :type Boolean))
  (Variables|Default|GetStatusUI
    (:then
      (if Visiblity
        (if (<= (Math|Vector|Distance(Vector) (Transformation|GetActorLocation (Variables|Default|GetPlayer)) (Transformation|GetActorLocation self)) 3e+03)
          (Widget|SetVisibility (Variables|Default|GetStatusUI) "Visible"))
        (else
          (Widget|SetVisibility (Variables|Default|GetStatusUI) "Hidden"))))
    (:else)))