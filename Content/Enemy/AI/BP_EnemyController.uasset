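; AI controller for BP_Enemy pawns that runs their behavior tree.
; On possess, it sets up the BB_Enemy blackboard, stores the pawn's current location as the base location, and starts BT_Enemy.
; Each tick, it checks the enemy's State and stops the brain logic while that matches one specific enum value.
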(event EventBeginPlay)

(event EventTick
  (params (DeltaSeconds :type Float%20%28single-precision%29))
  (bind _asbp_enemy (Utilities|Casting|CastToBP_Enemy (Pawn|GetControlledPawn)))
  (if (Utilities|Enum|Equal(Enum) (Variables|/Game/Enemy/BP_Enemy.BP_Enemy_C|GetState _asbp_enemy) "NewEnumerator1")
    (AI|Logic|StopLogic (Variables|Default|GetBrainComponent) "")))

(event EventPossess
  (params (PossessedPawn :type Pawn%20Object%20Reference))
  (bind _blackboardcomponent (Class|AIController|UseBlackboard "/Game/Enemy/AI/BB_Enemy.BB_Enemy"))
  (AI|Components|Blackboard|SetValueasVector _blackboardcomponent (Variables|Default|GetBaseLocationKey) (Transformation|GetActorLocation (Pawn|GetControlledPawn)))
  (AI|RunBehaviorTree "/Game/Enemy/AI/BT_Enemy.BT_Enemy"))

(fn ConstructionScript)