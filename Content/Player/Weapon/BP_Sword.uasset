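; BP_Sword is the player's melee weapon, which sets the player pawn as its owner on BeginPlay.
; While the player is attacking, overlapping a BP_Enemy deals fixed damage through its damage component, updates its health bar and shakes the camera.
; DefendEffect spawns a hit emitter at the sword's arrow, while ParryEffect briefly slows global time before reusing that path, which restores normal speed after a delay.
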(event Custom|ParryEffect
  (Utilities|Time|SetGlobalTimeDilation 0.7)
  (Utilities|FlowControl|Delay 0.2)
  (Effects|SpawnEmitteratLocation "/Game/Assets/TrailPack/Particles/Speed/Hit/P_SpeedHit.P_SpeedHit" (Transformation|GetWorldLocation (Variables|Default|GetArrow)))
  (Utilities|FlowControl|Delay 0.6)
  (Utilities|Time|SetGlobalTimeDilation 1.0))

(event Custom|DefendEffect
  (Effects|SpawnEmitteratLocation "/Game/Assets/TrailPack/Particles/Speed/Hit/P_SpeedHit.P_SpeedHit" (Transformation|GetWorldLocation (Variables|Default|GetArrow)))
  (Utilities|FlowControl|Delay 0.6)
  (Utilities|Time|SetGlobalTimeDilation 1.0))

(event EventBeginPlay
  (Actor|SetOwner (Game|Player|GetPlayerPawn 0))
  (bind _asbp_player (Utilities|Casting|CastToBP_Player (Components|GetOwner)))
  (Variables|Default|SetPlayer _asbp_player))

(event Collision|EventActorBeginOverlap
  (params (OtherActor :type Actor%20Object%20Reference))
  (if (Variables|/Game/Player/BP_Player.BP_Player_C|GetOnAttack (Variables|Default|GetPlayer))
    (bind _asbp_enemy (Utilities|Casting|CastToBP_Enemy OtherActor))
    (Default|GetDamage (Variables|/Game/Enemy/BP_Enemy.BP_Enemy_C|GetBP_DamageSystem _asbp_enemy) 1e+01 (Variables|Default|GetPlayer))
    (Default|SetTargetPercent (Variables|/Game/Enemy/BP_Enemy.BP_Enemy_C|GetStatusUI _asbp_enemy) (/ (Variables|/Game/Component/BP_DamageSystem.BP_DamageSystem_C|GetHealth%20Point (Variables|/Game/Enemy/BP_Enemy.BP_Enemy_C|GetBP_DamageSystem _asbp_enemy)) 1e+02))
    (CameraShakes|StartCameraShake (Game|GetPlayerCameraManager 0) "/Game/Player/BP_AttackCS.BP_AttackCS_C" 1.0 "CameraLocal" "0, 0, 0")))

(event EventTick
  (params (DeltaSeconds :type Float%20%28single-precision%29)))

(fn ConstructionScript)