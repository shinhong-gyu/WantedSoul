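; BP_DamageSystem is a component that tracks health, hit and death state for the actor it is attached to.
; On BeginPlay it caches its owner as a Character.
; GetDamage stores the instigator, subtracts damage from HealthPoint and raises the Hit flag, then sets Dead once health reaches zero or below.
; It only sets these variables, with no clamping, flag reset or reaction logic of its own.
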(event EventBeginPlay
  (bind _ascharacter (Utilities|Casting|CastToCharacter (Components|GetOwner)))
  (Variables|Default|SetOwner _ascharacter))

(event EventTick
  (params (DeltaSeconds :type Float%20%28single-precision%29)))

(fn GetDamage
  (params (Damage :type Float%20%28double-precision%29) (Instigator :type Actor%20Object%20Reference))
  (LocalVariables|SetInstigateActor Instigator)
  (bind _output_get (Variables|Default|SetHealth%20Point (- (Variables|Default|GetHealth%20Point) Damage)))
  (Variables|Default|SetbHit true)
  (if (<= _output_get 0.0)
    (Variables|Default|SetbDead true)))